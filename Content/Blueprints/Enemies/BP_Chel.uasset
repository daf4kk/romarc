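; BP_Chel is an enemy with health that reacts differently to ray damage and to other damage.
; DT_Ray damage costs no health and instead swaps every skeletal mesh material to an X-ray glow, restored after a retriggerable one-second delay.
; The original materials are cached in the construction script for that restore.
; Other damage reduces health, printing the remainder or destroying the actor once it is depleted.
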(event EventBeginPlay)

(event Collision|EventActorBeginOverlap
  (params (OtherActor :type Actor%20Object%20Reference)))

(event EventTick
  (params (DeltaSeconds :type Float%20%28single-precision%29)))

(event Game|Damage|EventAnyDamage
  (params (Damage :type Float%20%28single-precision%29) (DamageType :type Damage%20Type%20Object%20Reference) (InstigatedBy :type Controller%20Object%20Reference) (DamageCauser :type Actor%20Object%20Reference))
  (Utilities|Casting|CastToDT_Ray DamageType
    (:then
      (CallFunction|SetGlow)
      (Utilities|FlowControl|RetriggerableDelay 1.0)
      (CallFunction|RemoveGlow)
      (Development|PrintString "Hello"))
    (:CastFailed
      (bind _output_get (Variables|Default|SetCurrentHealth (- (Variables|Default|GetCurrentHealth) Damage)))
      (if (> _output_get 0.0)
        (Development|PrintString (Utilities|String|ToString(Float) (Variables|Default|GetCurrentHealth)))
        (else
          (Actor|DestroyActor))))))

(fn ConstructionScript
  (Variables|Default|SetSkeletalMaterials (Rendering|Material|GetMaterials (Variables|Default|GetSkeletalMesh))))

(fn SetGlow
  (for _index (range 0 (Utilities|Array|Length (Rendering|Material|GetMaterials (Variables|Default|GetSkeletalMesh))))
    (Rendering|Material|SetMaterial (Variables|Default|GetSkeletalMesh) _index "/Game/Blueprints/Materials/M_X-Ray2_Inst.M_X-Ray2_Inst")))

(fn RemoveGlow
  (for _index (range 0 (Utilities|Array|Length (Rendering|Material|GetMaterials (Variables|Default|GetSkeletalMesh))))
    (Rendering|Material|SetMaterial (Variables|Default|GetSkeletalMesh) _index (Utilities|Array|Get(acopy) (Variables|Default|GetSkeletalMaterials) _index))))