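; BP_AlphaRedan is the Alpha Redan AI character, which carries an arc sword and feeds its movement direction to animation.
; BeginPlay caches its ABP_AlphaRedan anim instance, then spawns BP_ArcSword snapped to the mesh's unsheath socket.
; Each Tick, it refreshes the direction through the parent's MoveDirection while moving and passes it to the Anim Blueprint.
; When stationary, it keeps sending the last stored direction.
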(event EventBeginPlay
  ;[1 0.2448 0.2448] Begin play
  (|CallParentFunction)
  (Utilities|FlowControl|Sequence
    (:then_0
      ;[1 1 1] start
      (bind _asabp_alpha_redan (Utilities|Casting|CastToABP_AlphaRedan (Components|SkeletalMesh|GetAnimInstance (Variables|Character|GetMesh))))
      (Variables|Default|SetABPAlphaRedan _asabp_alpha_redan)
      (bind _returnvalue (Game|SpawnActorfromClass "/Game/Blueprints/EquipActors/BP_ArcSword.BP_ArcSword_C" (Math|Transform|MakeTransform (Transformation|GetActorLocation) "0, 0, 0" "1.000000,1.000000,1.000000") "Undefined" 0 0))
      (Transformation|AttachComponentToComponent _returnvalue (Variables|Character|GetMesh) "UnsheathSocketArcSword" "SnapToTarget" "SnapToTarget" "SnapToTarget" true))))

(event Collision|EventActorBeginOverlap
  (params (OtherActor :type Actor%20Object%20Reference))
  (|CallParentFunction OtherActor) ; This node is disabled and will not be called.\nDrag off pins to build functionality.
)

(event EventTick
  (params (DeltaSeconds :type Float%20%28single-precision%29))
  (|CallParentFunction DeltaSeconds)
  (if (!= (Math|Vector|VectorLength (Transformation|GetVelocity)) 0.0)
    (CallFunction|MoveDirection)
    (Default|MoveDirection (Variables|Default|GetABPAlphaRedan) (Variables|Default|GetMoveDirectionAlphaRedan))
    (else
      (Default|MoveDirection (Variables|Default|GetABPAlphaRedan) (Variables|Default|GetMoveDirectionAlphaRedan)))))

(fn ConstructionScript
  (|CallParentFunction))

(fn MoveDirection
  (bind _outputdirection (|CallParentFunction))
  (Variables|Default|SetMoveDirectionAlphaRedan _outputdirection))