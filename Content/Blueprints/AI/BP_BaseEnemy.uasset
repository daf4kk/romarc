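; Base enemy character that tracks health, sets its run speed, records whoever damages it as its target, and is destroyed at zero health.
; Ray-type damage costs no health; it swaps all mesh materials to an X-ray material, then restores those cached in construction after a retriggerable one-second delay.
; MoveDirection returns the signed angle between velocity and facing.
; An AIMoveTo node is present but never runs.
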(event EventBeginPlay
  (Variables|EnemyStats|SetCurrentHealth (Variables|EnemyStats|GetMaxHealth))
  (Variables|/Script/Engine.CharacterMovementComponent|SetMaxWalkSpeed (Variables|Character|GetCharacterMovement) (Variables|EnemyStats|GetMaxRunSpeed)))

(event Game|Damage|EventAnyDamage
  (params (Damage :type Float%20%28single-precision%29) (DamageType :type Damage%20Type%20Object%20Reference) (InstigatedBy :type Controller%20Object%20Reference) (DamageCauser :type Actor%20Object%20Reference))
  (Utilities|Casting|CastToDT_Ray DamageType
    (:then
      (CallFunction|SetGlow)
      (Utilities|FlowControl|RetriggerableDelay 1.0)
      (CallFunction|RemoveGlow))
    (:CastFailed
      (bind _output_get (Variables|EnemyStats|SetCurrentHealth (- (Variables|EnemyStats|GetCurrentHealth) Damage)))
      (if (> _output_get 0.0)
        (Development|PrintString (Utilities|String|ToString(Float) (Variables|EnemyStats|GetCurrentHealth)))
        ;[1 1 1] Если получаем урон то заисываем актёра в таргер
        (Variables|EnemyStates|SetMobTarget DamageCauser)
        (else
          (Actor|DestroyActor))))))

(fn ConstructionScript
  (Variables|Materials|SetMeshMaterials (Rendering|Material|GetMaterials (Variables|Character|GetMesh))))

(fn SetGlow
  (for _index (range 0 (Utilities|Array|Length (Rendering|Material|GetMaterials (Variables|Character|GetMesh))))
    (Rendering|Material|SetMaterial (Variables|Character|GetMesh) _index "/Game/Materials/M_X-Ray2_Inst.M_X-Ray2_Inst")))

(fn RemoveGlow
  (for _index (range 0 (Utilities|Array|Length (Rendering|Material|GetMaterials (Variables|Character|GetMesh))))
    (Rendering|Material|SetMaterial (Variables|Character|GetMesh) _index (Utilities|Array|Get(acopy) (Variables|Materials|GetMeshMaterials) _index))))

(fn MoveDirection
  (bind _returnvalue (Transformation|GetVelocity))
  (bind _returnvalue_2 (Transformation|GetActorForwardVector))
  (bind _output_get (Variables|ABP|SetDirection (* (Class|KismetMathLibrary|DegAcos (Math|Vector|DotProduct (Math|Vector|Normalize _returnvalue) _returnvalue_2)) (Math|Float|Sign(Float) (.z (Math|Vector|CrossProduct _returnvalue _returnvalue_2))))))
  (return _output_get))