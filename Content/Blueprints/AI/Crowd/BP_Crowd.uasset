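; BP_Crowd is a crowd AI character that drops as a ragdoll when it collides with a BP_BaseCharacter.
; Each tick it refreshes its move direction through the parent's calculation while moving and passes the stored value to its ABP_Enemy anim instance, cached at BeginPlay.
; A qualifying capsule hit destroys the capsule, turns on mesh physics and destroys the actor after a short delay.
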(event OnComponentHit(CapsuleComponent)
  (params (HitComponent :type Primitive%20Component%20Object%20Reference) (OtherActor :type Actor%20Object%20Reference) (OtherComp :type Primitive%20Component%20Object%20Reference) (NormalImpulse :type Vector :default "0, 0, 0") (Hit :type Hit%20Result%20Structure%20%28by%20ref%29))
  (Utilities|Casting|CastToBP_BaseCharacter OtherActor)
  (Components|DestroyComponent (Variables|Default|GetCapsuleComponent))
  (Physics|SetSimulatePhysics (Variables|Character|GetMesh) true)
  (Utilities|FlowControl|Delay 3.0)
  (Actor|DestroyActor))

(event EventPossessed
  (params (NewController :type Controller%20Object%20Reference)))

(event Collision|EventActorBeginOverlap
  (params (OtherActor :type Actor%20Object%20Reference))
  (|CallParentFunction OtherActor) ; This node is disabled and will not be called.\nDrag off pins to build functionality.
)

(event EventTick
  (params (DeltaSeconds :type Float%20%28single-precision%29))
  (|CallParentFunction DeltaSeconds)
  (if (!= (Math|Vector|VectorLength (Transformation|GetVelocity)) 0.0)
    (CallFunction|MoveDirection)
    (Default|MoveDirection (Variables|Default|GetABPEnemyLox) (Variables|Default|GetMoveDirectionLox))
    (else
      (Default|MoveDirection (Variables|Default|GetABPEnemyLox) (Variables|Default|GetMoveDirectionLox)))))

(event EventBeginPlay
  (bind _asabp_enemy (Utilities|Casting|CastToABP_Enemy (Components|SkeletalMesh|GetAnimInstance (Variables|Character|GetMesh))))
  (Variables|Default|SetABPEnemyLox _asabp_enemy))

(fn ConstructionScript
  (|CallParentFunction))

(fn MoveDirection
  (bind _outputdirection (|CallParentFunction))
  (Variables|Default|SetMoveDirectionLox _outputdirection))