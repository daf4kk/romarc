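; AI controller Blueprint that serves as a sandbox for navigation experiments, with most movement logic disconnected.
; BeginPlay stores a random navigable point near the controlled pawn, and Tick casts a forward navmesh raycast without using the result.
; Unwired snippets try random roaming, looping through TargetPoints, moving to the player, and trace-based steering, so the controller issues no movement.
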(event EventTick
  (params (DeltaSeconds :type Float%20%28single-precision%29))
  (bind _returnvalue (Pawn|GetControlledPawn))
  (bind _returnvalue_2 (Transformation|GetActorLocation _returnvalue))
  ;[1 1 1] Проверяет на наличие границы navmesh перед собой
  (Class|NavigationSystemV1|NavigationRaycast _returnvalue_2 (+ _returnvalue_2 (* (Transformation|GetActorForwardVector _returnvalue) 3e+03)) 0 0))

(event EventBeginPlay
  ;[1 1 1] Random move
  (bind _randomlocation (Class|NavigationSystemV1|GetRandomLocationinNavigableRadius (Transformation|GetActorLocation (Pawn|GetControlledPawn)) 2e+02 0 0))
  (Variables|Default|SetRandomPoint _randomlocation))

(fn ConstructionScript)