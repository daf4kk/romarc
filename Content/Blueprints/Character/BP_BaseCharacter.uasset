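; Base player character with Enhanced Input movement, sword combat, and a toggleable monocle ability.
; Attacks and jumps spend regenerating stamina shown with health on the HUD, while movement and weapon state feed ABP_Character.
; Sword swaps are gated by montage-timed delays, and melee hits use a timer-driven socket trace that stops on first enemy hit.
; The monocle slows walking, fires a ricocheting damage ray with Niagara beams, and sphere-traces nearby walls, damaging them to see through.
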(event Custom|StartSphereOverla
  ;[1 0.4531 0.4531] Monocle Sphere (гг находится в сфере, при оверлапе она просвечивает стены)
  (bind _returnvalue (Utilities|Time|SetTimerbyEvent (delegate Custom|SphereOverlap) 0.01 true 1.0))
  (Variables|Default|SetSphereOverlapLoop _returnvalue))

(event Custom|EndSphereOverlap
  ;[1 0.4531 0.4531] Monocle Sphere (гг находится в сфере, при оверлапе она просвечивает стены)
  (Utilities|Time|ClearandInvalidateTimerbyHandle (Variables|Default|GetSphereOverlapLoop)))

(event Custom|SphereOverlap
  (bind _mesh (Variables|Character|GetMesh))
  (bind _returnvalue (Transformation|GetSocketLocation _mesh "pelvis"))
  ;[1 0.4531 0.4531] Monocle Sphere (гг находится в сфере, при оверлапе она просвечивает стены)
  (bind _outhits (Collision|MultiSphereTraceByChannel _returnvalue _returnvalue 2.5e+02 "TraceTypeQuery1" false 0 "None"))
  (for _array_element _outhits
    (bind _asbp_wall (Utilities|Casting|CastToBP_Wall (.HitActor (Collision|BreakHitResult _array_element))))
    (Game|Damage|ApplyDamage _asbp_wall 1e+01 0 0)))

(event Custom|StartSwordTrace
  ;[1 0.1823 0.1823] Sword trace
  (bind _returnvalue (Utilities|Time|SetTimerbyEvent (delegate Custom|SwordTraceLoop) 0.01 true))
  (Variables|Default|SetSwordTraceLoopVar _returnvalue))

(event Custom|SwordTraceLoop
  (bind _mesh (Variables|Character|GetMesh))
  (bind _returnvalue (Transformation|GetSocketLocation _mesh "TraceSocket"))
  ;[1 0.1823 0.1823] Sword trace
  (bind _outhit (Collision|SphereTraceForObjects _returnvalue _returnvalue 9e+01 (Utilities|Array|MakeArray "ObjectTypeQuery8") false 0 "ForDuration"))
  (bind _asbp_base_enemy (Utilities|Casting|CastToBP_BaseEnemy (.hitactor _outhit)))
  (Game|Damage|ApplyDamage _asbp_base_enemy (Variables|/Game/Blueprints/EquipActors/BP_BaseWeapon.BP_BaseWeapon_C|GetDamage (Variables|Weapons|GetCurrentWeapon)) 0 self)
  ;;[1 1 1 1 12] Если задели врага то отключаем trace что бы урон засчитывался 1 раз
  (CallFunction|StopSwordTrace))

(event Custom|StopSwordTrace
  ;[1 0.1823 0.1823] Sword trace
  (Utilities|Time|ClearandInvalidateTimerbyHandle (Variables|Default|GetSwordTraceLoopVar)))

(event Input|EnhancedActionEvents|EnhancedInputActionIA_Move
  (params (ActionValue :type Vector%202D%20Structure) (ElapsedSeconds :type Float%20%28double-precision%29) (TriggeredSeconds :type Float%20%28double-precision%29) (InputAction :type Input%20Action%20Object%20Reference :default "/Game/Blueprints/Input/Actions/IA_Move.IA_Move"))
  ;[0.0356 0 1] Movement/Camera
  (:Triggered
    (Pawn|Input|AddMovementInput (Transformation|GetActorForwardVector) (.x ActionValue) false)
    (Pawn|Input|AddMovementInput (Transformation|GetActorRightVector) (.y ActionValue) false)))

(event Input|EnhancedActionEvents|EnhancedInputActionIA_Look
  (params (ActionValue :type Vector%202D%20Structure) (ElapsedSeconds :type Float%20%28double-precision%29) (TriggeredSeconds :type Float%20%28double-precision%29) (InputAction :type Input%20Action%20Object%20Reference :default "/Game/Blueprints/Input/Actions/IA_Look.IA_Look"))
  ;[0.0356 0 1] Movement/Camera
  (:Triggered
    (Pawn|Input|AddControllerYawInput (.x ActionValue)) ; Turn
    (Utilities|FlowControl|Sequence
      (:then_0
        ;;[0.9876 0.3939 1] TurnInPlaceBoolean
        (if (== (Math|Vector|VectorLength (Transformation|GetVelocity)) 0.0)
          (Utilities|FlowControl|Sequence
            (:then_0
              (if (> (stale Input|MouseEvents|MouseX AxisValue) 0.5)
                (Utilities|TurnRight/Left? true false)
                (else
                  (Variables|Movement|SetisTurnRight false))))
            (:then_1
              (if (< (stale Input|MouseEvents|MouseX AxisValue) -0.5)
                (Utilities|TurnRight/Left? false true)
                (else
                  (Variables|Movement|SetIsTurnLeft false)))))
          (else
            (Utilities|TurnRight/Left? false false))))
      (:then_1
        (Pawn|Input|AddControllerPitchInput (* (.y ActionValue) -1.0)) ; Up
      ))))

(event Input|EnhancedActionEvents|EnhancedInputActionIA_EquipToughSword
  (params (ActionValue :type Boolean) (ElapsedSeconds :type Float%20%28double-precision%29) (TriggeredSeconds :type Float%20%28double-precision%29) (InputAction :type Input%20Action%20Object%20Reference :default "/Game/Blueprints/Input/Actions/IA_EquipToughSword.IA_EquipToughSword"))
  ;[0.1419 1 0.5265] Equip/Un weapon
  (:Started
    (Utilities|IsValid (Variables|Weapons|GetToughSword)
      (:Is%20Valid
        (if (Variables|CanWe|GetCanSwapWeapon)
          ;;[0 1 0.7617] Как либо взаимодействовать с оружием мы можем только в том случае, если
          ;; !current weapon || CurWea == "self"
          (if (or (not (Utilities|IsValid (Variables|Weapons|GetCurrentWeapon))) (== (Variables|Weapons|GetToughSword) (Variables|Weapons|GetCurrentWeapon)))
            _
            (else
              (Variables|CanWe|SetCanSwapWeapon false)
              (Variables|CanWe|SetCanAttack false)
              (bind _montagelength (Default|UnequipMontage (Variables|Weapons|GetCurrentWeapon)))
              (Utilities|FlowControl|Delay (/ _montagelength 1.5)) ; У нас оба shealth имеют общий тайминг\nно нужно передавать динамическм
              (Variables|CanWe|SetCanSwapWeapon true)))
          (Variables|CanWe|SetCanSwapWeapon false)
          (Variables|CanWe|SetCanAttack false)
          (bind _output_get (Variables|Weapons|SetCurrentWeapon (Variables|Weapons|GetToughSword)))
          (if (Default|GetIsAttachedtoHand _output_get)
            (bind _returnvalue (Animation|PlayAnimMontage "/Game/Animations/Montages/ArcSword/AM_ArcSword_Shealth.AM_ArcSword_Shealth" 1.5 "None"))
            (Utilities|FlowControl|Delay (/ _returnvalue 1.5))
            (Variables|CanWe|SetCanSwapWeapon true)
            (Variables|CanWe|SetCanAttack true)
            (CallFunction|SetABPWeaponTypebyCurrentWeapon)
            (else
              (bind _returnvalue_2 (Animation|PlayAnimMontage "/Game/Animations/Montages/ArcSword/AM_ArcSword_UnShealth.AM_ArcSword_UnShealth" 1.5 "None")) ; Un
              (Utilities|FlowControl|Delay (/ _returnvalue_2 1.5))
              (Variables|CanWe|SetCanSwapWeapon true)
              (Variables|CanWe|SetCanAttack true)
              (CallFunction|SetABPWeaponTypebyCurrentWeapon)))))
      (:Is%20Not%20Valid
        (Development|PrintString "Не валидный")))))

(event Input|EnhancedActionEvents|EnhancedInputActionIA_Interact
  (params (ActionValue :type Boolean) (ElapsedSeconds :type Float%20%28double-precision%29) (TriggeredSeconds :type Float%20%28double-precision%29) (InputAction :type Input%20Action%20Object%20Reference :default "/Game/Blueprints/Input/Actions/IA_Interact.IA_Interact"))
  (bind _returnvalue (Transformation|GetActorLocation))
  ;[1 0.9311 0.3291] PickUp
  (:Started
    (bind (_outhit _returnvalue_2) (Collision|SphereTraceForObjects _returnvalue _returnvalue 1e+02 (Utilities|Array|MakeArray "ObjectTypeQuery7") false 0 "None"))
    (if _returnvalue_2
      (Class|BPIInteract|Interact(Message) (.HitActor (Collision|BreakHitResult _outhit)) self))))

(event Input|EnhancedActionEvents|EnhancedInputActionIA_EquipGreatSword
  (params (ActionValue :type Boolean) (ElapsedSeconds :type Float%20%28double-precision%29) (TriggeredSeconds :type Float%20%28double-precision%29) (InputAction :type Input%20Action%20Object%20Reference :default "/Game/Blueprints/Input/Actions/IA_EquipGreatSword.IA_EquipGreatSword"))
  ;[0.1419 1 0.5265] Equip/Un weapon
  (:Started
    (Utilities|IsValid (Variables|Weapons|GetGreatSword)
      (:Is%20Valid
        (if (Variables|CanWe|GetCanSwapWeapon)
          (if (or (not (Utilities|IsValid (Variables|Weapons|GetCurrentWeapon))) (== (Variables|Weapons|GetGreatSword) (Variables|Weapons|GetCurrentWeapon)))
            _
            (else
              (Variables|CanWe|SetCanSwapWeapon false)
              (Variables|CanWe|SetCanAttack false)
              (bind _montagelength (Default|UnequipMontage (Variables|Weapons|GetCurrentWeapon)))
              (Utilities|FlowControl|Delay (/ _montagelength 1.5))
              (Variables|CanWe|SetCanSwapWeapon true)))
          (Variables|CanWe|SetCanSwapWeapon false)
          (Variables|CanWe|SetCanAttack false)
          (bind _output_get (Variables|Weapons|SetCurrentWeapon (Variables|Weapons|GetGreatSword)))
          (if (Default|GetIsAttachedtoHand _output_get)
            (bind _returnvalue (Animation|PlayAnimMontage "/Game/Animations/Montages/GreatSword/AM_GreatSword_Shealth.AM_GreatSword_Shealth" 1.0 "None"))
            (Utilities|FlowControl|Delay (/ _returnvalue 1.5))
            (Variables|CanWe|SetCanSwapWeapon true)
            (Variables|CanWe|SetCanAttack true)
            (CallFunction|SetABPWeaponTypebyCurrentWeapon)
            (else
              (bind _returnvalue_2 (Animation|PlayAnimMontage "/Game/Animations/Montages/GreatSword/AM_GreatSword_UnShealth.AM_GreatSword_UnShealth" 1.0 "None")) ; Un
              (Utilities|FlowControl|Delay (/ _returnvalue_2 1.5))
              (Variables|CanWe|SetCanSwapWeapon true)
              (Variables|CanWe|SetCanAttack true)
              (CallFunction|SetABPWeaponTypebyCurrentWeapon))))))))

(event Input|EnhancedActionEvents|EnhancedInputActionIA_Jump
  (params (ActionValue :type Boolean) (ElapsedSeconds :type Float%20%28double-precision%29) (TriggeredSeconds :type Float%20%28double-precision%29) (InputAction :type Input%20Action%20Object%20Reference :default "/Game/Blueprints/Input/Actions/IA_Jump.IA_Jump"))
  ;[0.0356 0 1] Movement/Camera
  (:Started
    (bind _isenough (Utilities|IsEnoughStamina (Variables|StaminaCost|GetJumpCost))
      (:ReturnValue
        (if (and _isenough (not (AI|Components|NavMovement|IsFalling (Variables|Character|GetCharacterMovement))))
          (Variables|PlayerStats|SetCurrentStamina (- (Variables|PlayerStats|GetCurrentStamina) (Variables|StaminaCost|GetJumpCost)))
          (Character|Jump)
          (Utilities|FlowControl|Delay 2.0))))))

(event Input|EnhancedActionEvents|EnhancedInputActionIA_Attack
  (params (ActionValue :type Boolean) (ElapsedSeconds :type Float%20%28double-precision%29) (TriggeredSeconds :type Float%20%28double-precision%29) (InputAction :type Input%20Action%20Object%20Reference :default "/Game/Blueprints/Input/Actions/IA_Attack.IA_Attack"))
  ;[1 0.4948 0.4948] Standart attack
  (:Started
    (Utilities|IsValid (Variables|Weapons|GetCurrentWeapon)
      (:Is%20Valid
        (if (Variables|CanWe|GetCanAttack)
          (bind _isenough (Utilities|IsEnoughStamina (Variables|StaminaCost|GetStandartAttackCost))
            (:ReturnValue
              (if _isenough
                (Variables|PlayerStats|SetCurrentStamina (- (Variables|PlayerStats|GetCurrentStamina) (Variables|StaminaCost|GetStandartAttackCost)))
                (CallFunction|UpdateStaminaHUD)
                (Variables|CanWe|SetCanAttack false)
                (bind _delay (Default|PlayAttackAnimation (Variables|Weapons|GetCurrentWeapon)))
                (Utilities|FlowControl|Delay (/ _delay 1.7))
                (Variables|CanWe|SetCanAttack true)))))))))

(event Input|EnhancedActionEvents|EnhancedInputActionIA_Monocle
  (params (ActionValue :type Boolean) (ElapsedSeconds :type Float%20%28double-precision%29) (TriggeredSeconds :type Float%20%28double-precision%29) (InputAction :type Input%20Action%20Object%20Reference :default "/Game/Blueprints/Input/Actions/IA_Monocle.IA_Monocle"))
  (bind _mesh (Variables|Character|GetMesh))
  (bind _camera (Variables|Components|GetCamera))
  (bind _monoclelength (Variables|Default|GetMonocleLength))
  (bind _returnvalue (Transformation|GetSocketLocation _mesh "MonocleSocket"))
  (bind _returnvalue_2 (Transformation|GetWorldTransform _camera))
  (bind _returnvalue_3 (Math|Vector|GetForwardVector (.rotation _returnvalue_2)))
  (bind _returnvalue_4 (* _returnvalue_3 _monoclelength))
  (bind _returnvalue_5 (+ (.location _returnvalue_2) _returnvalue_4))
  (:Started
    (Utilities|FlowControl|FlipFlop
      (:A
        ;[1 0.2334 0.7802] Monocle
        (bind _output_get (Variables|PlayerStates|SetInMonocle true))
        (Variables|/Script/Engine.CharacterMovementComponent|SetMaxWalkSpeed (Variables|Character|GetCharacterMovement) (Variables|Default|GetWalkSpeedInMonocle))
        (CallFunction|StartSphereOverla)
        (if _output_get :!label _label
          (bind _outhit (Collision|LineTraceByChannel _returnvalue _returnvalue_5 "TraceTypeQuery1" false 0 "None" true "(R=1.000000,G=0.000000,B=0.000000,A=1.000000)" "(R=0.000000,G=1.000000,B=0.000000,A=1.000000)" 0.2)) ; First Trace
          (CallFunction|TraceFX _returnvalue _returnvalue_5)
          (CallFunction|PerformTraceRicochet _outhit)
          (Utilities|FlowControl|Delay 0.001)
          (goto _label)))
      (:B
        (Variables|PlayerStates|SetInMonocle false)
        (Variables|/Script/Engine.CharacterMovementComponent|SetMaxWalkSpeed (Variables|Character|GetCharacterMovement) (Variables|Default|GetMaxWalkSpeed))
        (CallFunction|EndSphereOverlap)))))

(event EventTick
  (params (DeltaSeconds :type Float%20%28single-precision%29))
  ;[0 1 0.9823] Event tick
  (Utilities|FlowControl|Sequence
    (:then_0
      ;;[0.0356 0 1] Direction
      (if (!= (Math|Vector|VectorLength (Transformation|GetVelocity)) 0.0)
        (CallFunction|MoveDirection) ; Calculate direction
        (Default|MoveDirection (Variables|Default|GetABP_Ref) (Variables|Movement|GetDirection))
        (else
          (Default|MoveDirection (Variables|Default|GetABP_Ref) 0.0))))
    (:then_1
      ;;[0.2912 1 0.2907] Регенерация
      (Utilities|FlowControl|Delay 0.1)
      (if (< (Variables|PlayerStats|GetCurrentStamina) (Variables|PlayerStats|GetMaxStamina))
        (Variables|PlayerStats|SetCurrentStamina (+ (Variables|PlayerStats|GetCurrentStamina) (Variables|RegenRate|GetStaminaRegenRate)))
        (CallFunction|UpdateStaminaHUD)))))

(event Game|Damage|EventAnyDamage
  (params (Damage :type Float%20%28single-precision%29) (DamageType :type Damage%20Type%20Object%20Reference) (InstigatedBy :type Controller%20Object%20Reference) (DamageCauser :type Actor%20Object%20Reference))
  ;[1 0 0.1657] Take damage
  (Variables|PlayerStats|SetCurrentHealth (- (Variables|PlayerStats|GetCurrentHealth) Damage))
  (CallFunction|UpdateHPHUD)
  (Development|PrintString "ооо нет"))

(event EventBeginPlay
  ;[0 1 0.9823] Begin play
  ;;[0.03529 0 1] Enable mapping
  (bind _asbp_player_controller (Utilities|Casting|CastToBP_PlayerController (Game|GetPlayerController 0)))
  (Input|AddMappingContext (PlayerController|LocalPlayerSubsystems|GetEnhancedInputLocalPlayerSubsystem _asbp_player_controller) "/Game/Blueprints/Input/IMC_Character.IMC_Character" 0 "(bIgnoreAllPressedKeysUntilRelease=True,bForceImmediately=False)")
  ;;[0.03529 0 1] ABP Ref
  (bind _asabp_character (Utilities|Casting|CastToABP_Character (Components|SkeletalMesh|GetAnimInstance (Variables|Character|GetMesh))))
  (Variables|Default|SetABP_Ref _asabp_character)
  (bind _returnvalue (UserInterface|CreateWidget "/Game/HUD/WBP_CharacterHUD.WBP_CharacterHUD_C"))
  (bind _output_get (Variables|HUD|SetCharacterHUDRef _returnvalue))
  (UserInterface|Viewport|AddtoViewport _output_get 0)
  (Variables|PlayerStats|SetCurrentHealth (Variables|PlayerStats|GetMaxHealth))
  (Variables|PlayerStats|SetCurrentStamina (Variables|PlayerStats|GetMaxStamina)))

(event Input|MouseEvents|MouseX
  (params (AxisValue :type Float%20%28single-precision%29))
  ;[0.0356 0 1] Movement/Camera
  ;;[0.9876 0.3939 1] TurnInPlaceBoolean
)

(fn ConstructionScript)

(fn MoveDirection
  (bind _returnvalue (Transformation|GetVelocity))
  (bind _returnvalue_2 (Transformation|GetActorForwardVector))
  (Variables|Movement|SetDirection (* (Class|KismetMathLibrary|DegAcos (Math|Vector|DotProduct (Math|Vector|Normalize _returnvalue) _returnvalue_2)) (Math|Float|Sign(Float) (.z (Math|Vector|CrossProduct _returnvalue _returnvalue_2))))))

(fn SetABPWeaponTypebyCurrentWeapon
  (bind _abp_ref (Variables|Default|GetABP_Ref))
  (bind _currentweapon (Variables|Weapons|GetCurrentWeapon))
  (if (Utilities|IsValid _currentweapon)
    (Default|SetWeaponType _abp_ref (Variables|/Game/Blueprints/EquipActors/BP_BaseWeapon.BP_BaseWeapon_C|GetWeaponType _currentweapon))
    (else
      (Default|SetWeaponType _abp_ref "NewEnumerator0") ; Tough в расчёте на то, что его state является стандартным
    )))

(fn UnequipCurrentWeapon
  (params (current%20weapon :type BP%20Base%20Weapon%20Object%20Reference)))

(fn UpdateHPHUD
  (Progress|SetPercent (Variables|/Game/HUD/WBP_CharacterHUD.WBP_CharacterHUD_C|GetHealthBar (Variables|HUD|GetCharacterHUDRef)) (/ (Variables|PlayerStats|GetCurrentHealth) (Variables|PlayerStats|GetMaxHealth))))

(fn UpdateStaminaHUD
  (Progress|SetPercent (Variables|/Game/HUD/WBP_CharacterHUD.WBP_CharacterHUD_C|GetStaminaBar (Variables|HUD|GetCharacterHUDRef)) (/ (Variables|PlayerStats|GetCurrentStamina) (Variables|PlayerStats|GetMaxStamina))))

(fn TraceFX
  (params (StartPoint :type Vector) (EndPoint :type Vector))
  (bind _returnvalue (Niagara|SpawnSystematLocation (Variables|Default|GetTraceFXSystem) StartPoint))
  (Niagara|SetNiagaraVariable(Vector3) _returnvalue "TraceTarget" EndPoint))

(fn PerformTraceRicochet
  (params (StartingHit :type Hit%20Result%20Structure))
  ;[0 1 1 0.5] Perform line trace ricochet for each hit until the specified max limit
  (LocalVariables|SetLocal_PreviousHit StartingHit)
  (Utilities|FlowControl|ForLoopwithBreak 1 (Variables|PlayerStats|GetPlayerBoundsCount) :!label _label
    (:LoopBody
      (if (.bBlockingHit (Collision|BreakHitResult (LocalVariables|GetLocal_PreviousHit))) ; Did the previous trace operation generate a hit?
        (LocalVariables|SetNoImpactStart (+ (.ImpactPoint (Collision|BreakHitResult (LocalVariables|GetLocal_PreviousHit))) (Math|Vector|MirrorVectorbyNormal (Math|Vector|GetUnitDirection(Vector) (.TraceStart (Collision|BreakHitResult (LocalVariables|GetLocal_PreviousHit))) (.TraceEnd (Collision|BreakHitResult (LocalVariables|GetLocal_PreviousHit)))) (.ImpactNormal (Collision|BreakHitResult (LocalVariables|GetLocal_PreviousHit))))))
        (LocalVariables|SetNoImpactEnd (+ (.ImpactPoint (Collision|BreakHitResult (LocalVariables|GetLocal_PreviousHit))) (* (Math|Vector|MirrorVectorbyNormal (Math|Vector|GetUnitDirection(Vector) (.TraceStart (Collision|BreakHitResult (LocalVariables|GetLocal_PreviousHit))) (.TraceEnd (Collision|BreakHitResult (LocalVariables|GetLocal_PreviousHit)))) (.ImpactNormal (Collision|BreakHitResult (LocalVariables|GetLocal_PreviousHit)))) (Variables|Default|GetMonocleLength))))
        (bind _outhits (Collision|MultiLineTraceByChannel (+ (.ImpactPoint (Collision|BreakHitResult (LocalVariables|GetLocal_PreviousHit))) (Math|Vector|MirrorVectorbyNormal (Math|Vector|GetUnitDirection(Vector) (.TraceStart (Collision|BreakHitResult (LocalVariables|GetLocal_PreviousHit))) (.TraceEnd (Collision|BreakHitResult (LocalVariables|GetLocal_PreviousHit)))) (.ImpactNormal (Collision|BreakHitResult (LocalVariables|GetLocal_PreviousHit))))) (+ (.ImpactPoint (Collision|BreakHitResult (LocalVariables|GetLocal_PreviousHit))) (* (Math|Vector|MirrorVectorbyNormal (Math|Vector|GetUnitDirection(Vector) (.TraceStart (Collision|BreakHitResult (LocalVariables|GetLocal_PreviousHit))) (.TraceEnd (Collision|BreakHitResult (LocalVariables|GetLocal_PreviousHit)))) (.ImpactNormal (Collision|BreakHitResult (LocalVariables|GetLocal_PreviousHit)))) (Variables|Default|GetMonocleLength))) "TraceTypeQuery1" false 0 "None" true "(R=1.000000,G=0.000000,B=0.000000,A=1.000000)" "(R=0.000000,G=1.000000,B=0.000000,A=1.000000)" 0.1))
        (LocalVariables|SetLocal_PreviousHit "") ; Очищаем чтоб была корректная проверка \nна наличие стены в переменной
        (bind _array_element (Utilities|Array|ForEachLoopwithBreak _outhits :!label _label_2)
          (:LoopBody
            (bind _asbp_base_enemy (Utilities|Casting|CastToBP_BaseEnemy (.HitActor (Collision|BreakHitResult _array_element)))
              (:then
                (Game|Damage|ApplyDamage _asbp_base_enemy 1.0 0 0 "/Game/Blueprints/MonocleMechanics/DT_Ray.DT_Ray_C"))
              (:CastFailed
                (bind _output_get (LocalVariables|SetLocal_PreviousHit _array_element)) ; wall hit
                (bind _asbp_wall (Utilities|Casting|CastToBP_Wall (.HitActor (Collision|BreakHitResult _output_get))))
                (Game|Damage|ApplyDamage _asbp_wall 1e+01 0 0)
                (goto _label_2 Break))))
          (:Completed
            (if (.bBlockingHit (Collision|BreakHitResult (LocalVariables|GetLocal_PreviousHit)))
              ;[1 1 1] Impact point
              (CallFunction|TraceFX (.TraceStart (Collision|BreakHitResult (LocalVariables|GetLocal_PreviousHit))) (.ImpactPoint (Collision|BreakHitResult (LocalVariables|GetLocal_PreviousHit))))
              (else
                ;[1 1 1] Without impact
                (CallFunction|TraceFX (LocalVariables|GetNoImpactStart) (LocalVariables|GetNoImpactEnd))))))
        (else
          (goto _label Break))))))