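; BP_BaseWeapon is a base weapon equip actor that extends a parent equippable class and is owned by a BP_BaseCharacter.
; On BeginPlay it caches the owning character as PlayerRef, and it exposes a getter and setter for whether it is attached to the hand.
; OnEquip defers to the parent, while UnequipMontage plays nothing and returns a zero montage length with the cast owner.
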(event EventBeginPlay
  (|CallParentFunction)
  (bind _asbp_base_character (Utilities|Casting|CastToBP_BaseCharacter (Components|GetOwner)))
  (Variables|Default|SetPlayerRef _asbp_base_character))

(fn ConstructionScript
  (|CallParentFunction))

(fn SetIsAttachedtoHand
  (params (IsAttachToHand :type Boolean))
  (Variables|Default|SetIsAttachedToHand IsAttachToHand))

(fn GetIsAttachedtoHand
  (return (Variables|Default|GetIsAttachedToHand)))

(fn OnEquip
  (|CallParentFunction))

(fn UnequipMontage
  (bind _asbp_base_character (Utilities|Casting|CastToBP_BaseCharacter (Components|GetOwner)))
  (return 0.0 _asbp_base_character))