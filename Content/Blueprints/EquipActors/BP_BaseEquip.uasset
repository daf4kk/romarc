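; BP_BaseEquip is a base equippable item actor that tracks its equipped state and attaches to a character.
; Equipping sets the flag and snaps the item to SheathSocket on the owning BP_BaseCharacter's mesh through AttachActor, which accepts any socket.
; Unequipping only clears the flag, without detaching.
; GetItemMesh returns the static mesh component only when its mesh asset is invalid; its skeletal mesh return is unreachable.
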(fn ConstructionScript)

(fn GetItemMesh
  (Utilities|IsValid (Variables|/Script/Engine.StaticMeshComponent|GetStaticMesh (Variables|Default|GetItem_SM))
    (:Is%20Not%20Valid
      (return (Variables|Default|GetItem_SM)))))

(fn SetIsEquiped
  (params (IsEquiped :type Boolean))
  (Variables|Default|SetIsEquiped IsEquiped))

(fn GetIsEquiped
  (return (Variables|Default|GetIsEquiped)))

(fn OnEquip
  (Variables|Default|SetIsEquiped true)
  (CallFunction|AttachActor self (Variables|Default|GetSheathSocket)))

(fn OnUnequip
  (if (Variables|Default|GetIsEquiped)
    (Variables|Default|SetIsEquiped false)))

(fn AttachActor
  (params (SocketName :type Name))
  (bind _asbp_base_character (Utilities|Casting|CastToBP_BaseCharacter (Components|GetOwner)))
  (Transformation|AttachComponentToComponent self (Variables|/Script/Engine.Character|GetMesh _asbp_base_character) SocketName "SnapToTarget" "SnapToTarget" "SnapToTarget" true))