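; BP_GreatSword is the equippable great sword actor, overriding equip and sheathe behavior from its parent.
; On equip it runs the parent logic, then registers itself as the GreatSword on the owner's character, reached through CharacterRefMessage.
; Sheathing plays the great sword sheathe montage through the character's AnimBP reference.
; Unequip plays the same montage faster on the parent-supplied base character and returns its length.
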(event EventBeginPlay
  (|CallParentFunction) ; This node is disabled and will not be called.\nDrag off pins to build functionality.
)

(event Collision|EventActorBeginOverlap
  (params (OtherActor :type Actor%20Object%20Reference))
  (|CallParentFunction OtherActor) ; This node is disabled and will not be called.\nDrag off pins to build functionality.
)

(event EventTick
  (params (DeltaSeconds :type Float%20%28single-precision%29))
  (|CallParentFunction DeltaSeconds) ; This node is disabled and will not be called.\nDrag off pins to build functionality.
)

(fn ConstructionScript
  (|CallParentFunction))

(fn OnEquip
  (|CallParentFunction)
  (bind _character (Class|BPICharacter|CharacterRef(Message) (Components|GetOwner)))
  (Variables|/Game/Blueprints/Character/BP_BaseCharacter.BP_BaseCharacter_C|SetGreatSword _character self))

(fn ShealtWeapon
  (bind _character (Class|BPICharacter|CharacterRef(Message) (Components|GetOwner)))
  (Animation|Montage|MontagePlay (Variables|/Game/Blueprints/Character/BP_BaseCharacter.BP_BaseCharacter_C|GetABP_Ref _character) "/Game/Animations/Montages/GreatSword/AM_GreatSword_Shealth.AM_GreatSword_Shealth" 1.0 "MontageLength" 0.0 true))

(fn UnequipMontage
  (bind _asbp_base_character (|CallParentFunction))
  (bind _returnvalue (Animation|PlayAnimMontage _asbp_base_character "/Game/Animations/Montages/GreatSword/AM_GreatSword_Shealth.AM_GreatSword_Shealth" 1.5 "None"))
  (return _returnvalue 0))

(fn CharacterRef
  (return 0))