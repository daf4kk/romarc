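; Arc Sword equip actor that supplies the sword-specific animations for a character's equipment.
; On equip it registers itself as the owning BP_BaseCharacter's ArcSword.
; It extends parent functions to play the sheath montage for sheathing and unequipping (sped up for the latter), and randomly picks one of two attack montages.
; Attack and unequip return the montage play result as a timing value to the caller.
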(event EventBeginPlay
  (|CallParentFunction) ; This node is disabled and will not be called.\nDrag off pins to build functionality.
)

(event Collision|EventActorBeginOverlap
  (params (OtherActor :type Actor%20Object%20Reference))
  (|CallParentFunction OtherActor) ; This node is disabled and will not be called.\nDrag off pins to build functionality.
)

(event EventTick
  (params (DeltaSeconds :type Float%20%28single-precision%29))
  (|CallParentFunction DeltaSeconds) ; This node is disabled and will not be called.\nDrag off pins to build functionality.
)

(fn ConstructionScript
  (|CallParentFunction))

(fn OnEquip
  (|CallParentFunction)
  (bind _asbp_base_character (Utilities|Casting|CastToBP_BaseCharacter (Components|GetOwner)))
  (Variables|/Game/Blueprints/Character/BP_BaseCharacter.BP_BaseCharacter_C|SetArcSword _asbp_base_character self))

(fn ShealtWeapon
  (bind _character (Class|BPICharacter|CharacterRef(Message) (Components|GetOwner)))
  (Animation|Montage|MontagePlay (Variables|/Game/Blueprints/Character/BP_BaseCharacter.BP_BaseCharacter_C|GetABP_Ref _character) "/Game/Animations/Montages/ArcSword/AM_ArcSword_Shealth.AM_ArcSword_Shealth" 1.0 "MontageLength" 0.0 true))

(fn UnequipMontage
  (bind _asbp_base_character (|CallParentFunction))
  (bind _returnvalue (Animation|PlayAnimMontage _asbp_base_character "/Game/Animations/Montages/ArcSword/AM_ArcSword_Shealth.AM_ArcSword_Shealth" 1.5 "None"))
  (return _returnvalue 0))

(fn PlayAttackAnimation
  (bind _abp_ref (|CallParentFunction))
  (switch int (Math|Random|RandomIntegerinRange 0 1)
    (:0
      (bind _returnvalue (Animation|Montage|MontagePlay _abp_ref "/Game/Animations/Montages/ArcSword/AttackMontages/AM_ArcSword_Attack1.AM_ArcSword_Attack1" 1.0 "MontageLength" 0.0 true))
      (return 0 _returnvalue))
    (:1
      (bind _returnvalue_2 (Animation|Montage|MontagePlay _abp_ref "/Game/Animations/Montages/ArcSword/AttackMontages/AM_ArcSword_Attack2.AM_ArcSword_Attack2" 1.0 "MontageLength" 0.0 true))
      (return 0 _returnvalue_2))))

(fn CharacterRef
  (return 0))